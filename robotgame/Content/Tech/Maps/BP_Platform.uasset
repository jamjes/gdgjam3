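; BP_Platform is a moving platform that travels between its placed position and a configurable target.
; The construction script gives an InterpToMovement component two relative control points, the origin and TargetPosition, and applies MoveDuration.
; When the movement reverses, the event graph disables the component's tick for PauseAtDestination seconds, then re-enables it to resume motion.
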(event `self.ReceiveBeginPlay`)

(event `self.InterpToMovement.OnInterpToReverse`
  (params (ImpactResult :type "HitResult Structure (by ref)") (Time :type "Float (single-precision)"))
  (bind _interptomovement (`self.InterpToMovement`))
  (`ActorComponent.SetComponentTickEnabled` _interptomovement false)
  (`KismetSystemLibrary.Delay` (`self.PauseAtDestination`))
  (`ActorComponent.SetComponentTickEnabled` _interptomovement true))

(fn `UserConstructionScript`
  (bind _interptomovement (`self.InterpToMovement`))
  (`InterpToMovementComponent.AddControlPointPosition` _interptomovement (0.0 0.0 0.0) true)
  (`InterpToMovementComponent.AddControlPointPosition` _interptomovement (`self.TargetPosition`) true)
  (set `InterpToMovementComponent.Duration` (`self.MoveDuration`) _interptomovement))