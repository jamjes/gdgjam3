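; Side-scroller camera manager that follows the player character and drives parallax background layers.
; BeginPlay sets the spring arm length and gives each Paper sprite under BG a dynamic material with its own parallax multiplier.
; Each Tick eases the actor toward the player plus a facing-based X/Z offset, then feeds camera X to the layer materials for shader-side parallax.
; Spline-based Y positioning is stubbed out and never runs.
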(event `self.ReceiveBeginPlay`
  (set `self.FollowTarget` (`GameplayStatics.GetPlayerCharacter` 0))
  (set `SpringArmComponent.TargetArmLength` (`self.CameraDistance`) (`self.SpringArm`))
  (for (_array_element _array_index) (`SceneComponent.GetChildrenComponents` (`self.BG`) false)
    (bind _returnvalue (`PrimitiveComponent.CreateDynamicMaterialInstance` (cast `PaperSpriteComponent` _array_element :!pure true) 0 null "None"))
    (`KismetArrayLibrary.Array_Add` (`self.DynamicLayers`) _returnvalue)
    (`MaterialInstanceDynamic.SetScalarParameterValue` _returnvalue "ParallaxMultiplier" (`|GetArrayItem` (`self.ParallaxMultipliers`) _array_index))))

(event `self.ReceiveTick`
  (params (DeltaSeconds :type "Float (single-precision)"))
  (`self.UpdateCameraPosition`)
  (`self.ParallaxUpdate`))

(event `UseSplineY`)

(event `ParallaxUpdate`
  (bind _returnvalue_x (`KismetMathLibrary.BreakVector` (`SceneComponent.K2_GetComponentLocation` (`self.Camera`))))
  (for _array_element (`self.DynamicLayers`)
    (`MaterialInstanceDynamic.SetScalarParameterValue` _array_element "CameraPosX" _returnvalue_x)))

(fn `UpdateCameraPosition`
  (bind (_returnvalue_x _returnvalue_y _returnvalue_z) (`KismetMathLibrary.BreakVector` (`self.K2_GetActorLocation` (`self.FollowTarget`))))
  (bind (_returnvalue_x_2 _returnvalue_y_2 _returnvalue_z_2) (`KismetMathLibrary.BreakVector` (* (`self.GetActorForwardVector` (`self.FollowTarget`)) (`self.CameraOffset`))))
  (`self.K2_SetActorLocation` (`KismetMathLibrary.VInterpTo` (`self.K2_GetActorLocation`) (+ (`KismetMathLibrary.MakeVector` _returnvalue_x _returnvalue_y _returnvalue_z) (`KismetMathLibrary.MakeVector` _returnvalue_x_2 0.0 _returnvalue_z_2)) (`GameplayStatics.GetWorldDeltaSeconds`) (`self.FollowDelay`))))

(fn `UserConstructionScript`)