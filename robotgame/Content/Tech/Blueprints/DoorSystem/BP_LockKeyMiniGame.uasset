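; BP_LockKeyMiniGame is a trigger actor that runs a lock-in encounter cleared by destroying a set of doors.
; BeginPlay hides and disables the Doors and StartDoor, and binds each door's OnDoorDestroy event.
; When the player pawn overlaps it, it activates all doors and the StartDoor, then disables its own collision.
; A counter tracks destroyed doors; when all are gone, it hides StartDoor and destroys itself.
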(event `self.ReceiveActorBeginOverlap`
  (params (OtherActor :type "Actor Object Reference"))
  (bind _startdoor (`self.StartDoor`))
  (if (== OtherActor (`Controller.K2_GetPawn` (`GameplayStatics.GetPlayerController` 0)))
    (for _array_element (`self.Doors`)
      (`self.SetActorHiddenInGame` _array_element false)
      (`self.SetActorEnableCollision` _array_element true))
    (`self.SetActorHiddenInGame` _startdoor false)
    (`self.SetActorEnableCollision` _startdoor true)
    (`self.SetActorEnableCollision` false)))

(event `CheckArenaWin`
  (bind _destroycount (`self.destroycount`))
  (bind _startdoor (`self.StartDoor`))
  (`/Engine/EditorBlueprintResources/StandardMacros.IncrementInt` _destroycount
    (:`  `
      (if (== _destroycount (`KismetArrayLibrary.Array_Length` (`self.Doors`)))
        (`self.SetActorHiddenInGame` _startdoor true)
        (`self.SetActorEnableCollision` _startdoor false)
        (`self.K2_DestroyActor`)))))

(event `self.ReceiveBeginPlay`
  (bind _startdoor (`self.StartDoor`))
  (for _array_element (`self.Doors`)
    (add `/Game/Tech/Blueprints/BP_Door.OnDoorDestroy` _array_element (delegate `DoorDestroyed`))
    (`self.SetActorHiddenInGame` _array_element true)
    (`self.SetActorEnableCollision` _array_element false))
  (`self.SetActorHiddenInGame` _startdoor true)
  (`self.SetActorEnableCollision` _startdoor false))

(event `DoorDestroyed`
  (`self.CheckArenaWin`))

(fn `UserConstructionScript`)