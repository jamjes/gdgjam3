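; BP_CameraTrigger is a trigger actor that toggles a camera framing mode when the player's controlled pawn begins overlapping it.
; It finds the BP_CameraFramerSystem in the level and alternately sends it an enter message with its View value or an exit message.
; An Enter flag flips on each overlap, so leaving the trigger does nothing and every second entry exits the mode.
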(event `self.ReceiveActorBeginOverlap`
  (params (OtherActor :type "Actor Object Reference"))
  (if (== OtherActor (`Controller.K2_GetPawn` (`GameplayStatics.GetPlayerController` 0)))
    (bind _returnvalue (`GameplayStatics.GetActorOfClass` "/Game/Tech/Blueprints/BP_CameraFramerSystem.BP_CameraFramerSystem_C"))
    (if (`self.Enter`)
      (message `/Game/Tech/Blueprints/BPI_CameraSystem.EnterCameraMode` _returnvalue (`self.VIew`))
      (set `self.Enter` false)
      (else
        (message `/Game/Tech/Blueprints/BPI_CameraSystem.ExitCameraMode` _returnvalue)
        (set `self.Enter` true)))))

(fn `UserConstructionScript`)