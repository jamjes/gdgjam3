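; Button-mash trap that reveals blocking doors when the player's pawn overlaps it, picking a random key and showing it with a counter.
; Each press of that key lowers the counter, while a Delay on Tick periodically raises it.
; At zero the doors and trap are destroyed; at EndCondition BP_Game respawns the player and the doors hide.
; Start and both outcomes toggle pawn messages and switch BP_Game sounds.
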(event `self.ReceiveActorBeginOverlap`
  (params (OtherActor :type "Actor Object Reference"))
  (if (and (== OtherActor (`Controller.K2_GetPawn` (`GameplayStatics.GetPlayerController` 0))) (== (`self.Run`) false))
    (set `self.Run` true)
    (`self.Init`)
    (message `/Game/Tech/Blueprints/BPI_Pausable.Pause` (`Controller.K2_GetPawn` (`GameplayStatics.GetPlayerController` 0)))
    (bind _asbp_game (cast `/Game/Tech/Blueprints/BP_Game` (`GameplayStatics.GetGameMode`)))
    (`/Game/Tech/Blueprints/BP_Game.StopSound` _asbp_game)
    (`/Game/Tech/Blueprints/BP_Game.PlaySound` _asbp_game 1)))

(event `/Game/Tech/Blueprints/BPI_InputReader.OnKeyStart`
  (params (Key :type "InputAction Object Reference"))
  (if (== Key (`self.Target Key`))
    (bind _result (`/Engine/EditorBlueprintResources/StandardMacros.DecrementInt` (`self.Counter`))
      (:`  `
        (`self.UpdateUI`)
        (if (== _result 0)
          (for _array_element (`self.Door Reference`)
            (`self.K2_DestroyActor` _array_element))
          (`self.K2_DestroyActor`)
          (message `/Game/Tech/Blueprints/BPI_Pausable.Play` (`Controller.K2_GetPawn` (`GameplayStatics.GetPlayerController` 0)))
          (bind _asbp_game (cast `/Game/Tech/Blueprints/BP_Game` (`GameplayStatics.GetGameMode`)))
          (`/Game/Tech/Blueprints/BP_Game.StopSound` _asbp_game)
          (`/Game/Tech/Blueprints/BP_Game.PlaySound` _asbp_game 0))))))

(event `self.ReceiveBeginPlay`
  (`self.Hide`))

(event `self.ReceiveTick`
  (params (DeltaSeconds :type "Float (single-precision)"))
  (if (`self.Run`)
    (`KismetSystemLibrary.Delay` (`self.IncrementInterval`))
    (bind _result (`/Engine/EditorBlueprintResources/StandardMacros.IncrementInt` (`self.Counter`))
      (:`  `
        (`self.UpdateUI`)
        (if (== _result (`self.EndCondition`))
          (bind _asbp_game (cast `/Game/Tech/Blueprints/BP_Game` (`GameplayStatics.GetGameMode`)))
          (`/Game/Tech/Blueprints/BP_Game.RespawnPlayer` _asbp_game)
          (`self.Hide`)
          (message `/Game/Tech/Blueprints/BPI_Pausable.Play` (`Controller.K2_GetPawn` (`GameplayStatics.GetPlayerController` 0)))
          (bind _asbp_game_2 (cast `/Game/Tech/Blueprints/BP_Game` (`GameplayStatics.GetGameMode`)))
          (`/Game/Tech/Blueprints/BP_Game.StopSound` _asbp_game_2)
          (`/Game/Tech/Blueprints/BP_Game.PlaySound` _asbp_game_2 0))))))

(fn `Hide`
  (for _array_element (`self.Door Reference`)
    (`self.SetActorHiddenInGame` _array_element true)
    (`self.SetActorEnableCollision` _array_element false))
  (set `self.Run` false))

(fn `Init`
  (for _array_element (`self.Door Reference`)
    (`self.SetActorHiddenInGame` _array_element false)
    (`self.SetActorEnableCollision` _array_element true))
  (bind _output_get (set `self.Target Key` (`KismetArrayLibrary.Array_Random` (`self.All Keys`))))
  (`TextRenderComponent.K2_SetText` (`self.Key Label`) (`KismetTextLibrary.Conv_StringToText` (`KismetSystemLibrary.GetDisplayName` _output_get)))
  (set `self.Counter` (`self.MaxPress`))
  (`self.UpdateUI`))

(fn `UpdateUI`
  (`TextRenderComponent.K2_SetText` (`self.Counter Label`) (`KismetTextLibrary.Conv_IntToText` (`self.Counter`))))

(fn `UserConstructionScript`)