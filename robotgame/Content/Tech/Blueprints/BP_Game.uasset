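; BP_Game is a game-level manager that handles background sound and player respawning.
; On BeginPlay it starts the game sound, and PlaySound switches by index between the game and puzzle cues, spawning each as 2D audio stored as the current sound.
; StopSound deactivates that current sound if it is active.
; RespawnPlayer moves the player character to the respawn position of the last checkpoint.
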(event `self.ReceiveBeginPlay`
  (`self.PlaySound` 0))

(event `RespawnPlayer`
  (`self.K2_SetActorLocation` (`GameplayStatics.GetPlayerCharacter` 0) (`SceneComponent.K2_GetComponentLocation` (`/Game/Tech/Blueprints/BP_Checkpoint.RespawnPosition` (`self.LastCheckpoint`))) false false))

(fn `PlaySound`
  (params (SoundIndex :type Integer))
  (switch `int` SoundIndex
    (:`0`
      (bind _returnvalue (`GameplayStatics.SpawnSound2D` "/Game/Tech/Sounds/SC_Game.SC_Game" 1.0 1.0 0.0 null))
      (bind _output_get (set `self.CurerntSound` _returnvalue))
      (`ActorComponent.SetActive` _output_get true false))
    (:`1`
      (bind _returnvalue_2 (`GameplayStatics.SpawnSound2D` "/Game/Tech/Sounds/SC_Puzzle.SC_Puzzle" 1.0 1.0 0.0 null))
      (bind _output_get_2 (set `self.CurerntSound` _returnvalue_2))
      (`ActorComponent.SetActive` _output_get_2 true false))))

(fn `StopSound`
  (bind _curerntsound (`self.CurerntSound`))
  (if (`ActorComponent.IsActive` _curerntsound)
    (`ActorComponent.SetActive` _curerntsound false false)))

(fn `UserConstructionScript`)