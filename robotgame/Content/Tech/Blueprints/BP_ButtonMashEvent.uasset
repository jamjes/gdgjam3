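; BP_ButtonMashEvent is a trigger actor for a button-mash event that opens a referenced Door.
; Overlap with BP_ACO sets CanCount, and leaving clears it and resets the counter.
; IncrementCounter, which has no caller or CanCount check in this Blueprint, adds to Counter and, at a fixed threshold, opens the Door and destroys the trigger.
; Print strings announce the start, prompting the I key, and the completion.
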(event `self.ReceiveActorBeginOverlap`
  (params (OtherActor :type "Actor Object Reference"))
  (`KismetSystemLibrary.PrintString` "Mash Event Started! \nPRESS 'I'")
  (if (== (`GameplayStatics.GetObjectClass` OtherActor) "/Game/Tech/Blueprints/BP_ACO.BP_ACO_C")
    (set `self.CanCount` true)))

(event `self.ReceiveActorEndOverlap`
  (params (OtherActor :type "Actor Object Reference"))
  (if (== (`GameplayStatics.GetObjectClass` OtherActor) "/Game/Tech/Blueprints/BP_ACO.BP_ACO_C")
    (set `self.CanCount` false)
    (set `self.Counter` 0)))

(fn `IncrementCounter`
  (bind _result (`/Engine/EditorBlueprintResources/StandardMacros.IncrementInt` (`self.Counter`))
    (:`  `
      (if (== _result 20)
        (`/Game/Tech/Blueprints/BP_Door.Open` (`self.Door`) null)
        (`self.K2_DestroyActor`)
        (`KismetSystemLibrary.PrintString` "Button Mash Complete")))))

(fn `UserConstructionScript`)