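; Quick-time event trigger that traps the player behind doors until a random key sequence is entered or time runs out.
; Overlap by the player's pawn reveals the Door actors, builds and displays the key sequence, and starts a countdown driven by a one-second Delay on Tick.
; Matching presses advance a pointer; completion destroys the doors and trigger, while timeout respawns the player through BP_Game and hides the doors.
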(event `self.ReceiveBeginPlay`
  (`self.Hide`))

(event `self.ReceiveActorBeginOverlap`
  (params (OtherActor :type "Actor Object Reference"))
  (if (and (== OtherActor (`Controller.K2_GetPawn` (`GameplayStatics.GetPlayerController` 0))) (== (`self.Run`) false))
    (`self.Init`)
    (set `self.Run` true)))

(event `self.ReceiveTick`
  (params (DeltaSeconds :type "Float (single-precision)"))
  (bind _timeremaining (`self.TimeRemaining`))
  (if (`self.Run`)
    (`KismetSystemLibrary.Delay` 1.0)
    (`/Engine/EditorBlueprintResources/StandardMacros.DecrementFloat` _timeremaining
      (:`  `
        (`self.UpdateTimer`)
        (if (== _timeremaining 0.0)
          (`/Game/Tech/Blueprints/BP_Game.RespawnPlayer` (cast `/Game/Tech/Blueprints/BP_Game` (`GameplayStatics.GetGameMode`) :!pure true))
          (`self.Hide`))))))

(event `/Game/Tech/Blueprints/BPI_InputReader.OnKeyStart`
  (params (Key :type "InputAction Object Reference"))
  (bind _pointer (`self.Pointer`))
  (if (== Key (`|GetArrayItem` (`self.TargetKeys`) (`self.Pointer`)))
    (`/Engine/EditorBlueprintResources/StandardMacros.IncrementInt` _pointer
      (:`  `
        (if (== _pointer (`self.QTLengthKeys`))
          (for _array_element (`self.Door`)
            (`self.K2_DestroyActor` _array_element))
          (`self.K2_DestroyActor`))))))

(fn `Hide`
  (for _array_element (`self.Door`)
    (`self.SetActorHiddenInGame` _array_element true)
    (`self.SetActorEnableCollision` _array_element false))
  (set `self.Run` false)
  (set `self.TimeRemaining` (`self.Duration`)))

(fn `Init`
  (bind _targetkeys (`self.TargetKeys`))
  (set `self.KeysAsString` "")
  (for _array_element (`self.Door`)
    (`self.SetActorHiddenInGame` _array_element false)
    (`self.SetActorEnableCollision` _array_element true))
  (for _ (range (`self.QTLengthKeys`))
    (bind _returnvalue (`KismetArrayLibrary.Array_Add` _targetkeys (`KismetArrayLibrary.Array_Random` (`self.InputActions`))))
    (set `self.KeysAsString` (`KismetStringLibrary.Concat_StrStr` (`self.KeysAsString`) (`KismetSystemLibrary.GetDisplayName` (`|GetArrayItem` _targetkeys _returnvalue)) " \n"))
    (`self.UpdateTimer`))
  (`TextRenderComponent.K2_SetText` (`self.Key Label`) (`KismetTextLibrary.Conv_StringToText` (`self.KeysAsString`))))

(fn `UpdateTimer`
  (`TextRenderComponent.K2_SetText` (`self.Timer Label`) (`KismetTextLibrary.Conv_DoubleToText` (`self.TimeRemaining`) "HalfToEven")))

(fn `UserConstructionScript`)